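; Pistol weapon interactable that triggers the player's weapon pickup, plays a fire animation and spawns a projectile when fired.
; BulletTrace line-traces from the follow camera, damaging and dismembering hit zombies, or otherwise aiming the projectile transform from the muzzle arrow toward the impact or camera direction.
; Reload refills the clip from inventory ammo, which is initialized from clip size at construction.
; Recoil, ammo decrement and empty-clip message logic are disconnected.
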(event `self.ReceiveBeginPlay`
  (`parent.ReceiveBeginPlay`))

(event `FirePistol`
  (`SkeletalMeshComponent.PlayAnimation` (`self.InteractableSkeletalMesh`) "/Game/MilitaryWeapSilver/Weapons/Animations/Fire_Pistol_W.Fire_Pistol_W" false)
  (bind _spawntransfrom (`self.Bullet Trace`))
  (`|SpawnActorFromClass` "/Game/Blueprints/Projectiles/BP_PistolProjectile.BP_PistolProjectile_C" _spawntransfrom "AlwaysSpawn" "OverrideRootScale" null null))

(event `ReloadPistol`
  (if (< (`self.CurrentClipAmmo`) (`self.MaxClipAmmo`))
    (set `self.BulletDifference` (- (`self.MaxClipAmmo`) (`self.CurrentClipAmmo`)))
    (set `self.CurrentClipAmmo` (+ (`self.CurrentClipAmmo`) (`self.BulletDifference`)))
    (set `self.CurrentInventoryAmmo` (- (`self.CurrentInventoryAmmo`) (`self.BulletDifference`)))))

(fn `Bullet Trace`
  (returns (SpawnTransfrom :type "Transform Structure"))
  (bind (_outhit _camerarotation) (`self.LineTrace`))
  (bind _returnvalue (`SceneComponent.K2_GetComponentLocation` (`self.Arrow`)))
  (bind (_bblockinghit _binitialoverlap _time _distance _location _impactpoint _normal _impactnormal _physmat _hitactor _hitcomponent _hitbonename) (`GameplayStatics.BreakHitResult` _outhit))
  (bind _asbp_master_zombie (cast `/Game/Blueprints/Core/Enemy/BP_MasterZombie` _hitactor)
    (:`then`
      (`/Game/Blueprints/Core/Enemy/BP_MasterZombie.AffectHealth` _asbp_master_zombie -20.0)
      (bind (_limbtodismember _hitdismember_) (`/Game/Blueprints/Core/Enemy/BP_MasterZombie.GetDamagedLimb` _asbp_master_zombie))
      (if _hitdismember_
        (`/Game/Blueprints/Core/Enemy/BP_MasterZombie.DamageLimb` _asbp_master_zombie _limbtodismember)))
    (:`CastFailed`
      (return (`KismetMathLibrary.MakeTransform` _returnvalue (select `bool` _bblockinghit :`false` _camerarotation :`true` (`KismetMathLibrary.FindLookAtRotation` _returnvalue _impactpoint)))))))

(fn `Interact`
  (params (PlayerReference :type "/Game/Blueprints/Core/Player/BP_Player Object Reference"))
  (`parent.Interact` PlayerReference)
  (`/Game/Blueprints/Core/Player/BP_Player.WeaponsPickup` PlayerReference))

(fn `LineTrace`
  (returns (OutHit :type "HitResult Structure") (CameraRotation :type "Rotator Structure"))
  (bind _followcamera (`/Game/Blueprints/Core/Player/BP_Player.FollowCamera` (`self.PlayerReference`)))
  (bind _returnvalue (`SceneComponent.K2_GetComponentLocation` _followcamera))
  (bind _outhit (`KismetSystemLibrary.LineTraceSingle` :`Start` _returnvalue :`End` (+ _returnvalue (* (`SceneComponent.GetForwardVector` _followcamera) 15000.0)) :`TraceChannel` "TraceTypeQuery1" :`DrawDebugType` "ForDuration" :`DrawTime` 2.0))
  (return _outhit (`SceneComponent.K2_GetComponentRotation` _followcamera)))

(fn `UserConstructionScript`
  (`parent.UserConstructionScript`)
  (bind _output_get (set `self.MaxInventoryAmmo` (* (`self.MaxClipAmmo`) (`self.ClipMultiplier`))))
  (set `self.CurrentInventoryAmmo` _output_get))