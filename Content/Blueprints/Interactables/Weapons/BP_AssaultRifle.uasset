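; Interactable assault rifle that calls the player's weapon pickup on interact and fires using pistol-named event, animation and projectile.
; BulletTrace line-traces from the follow camera with debug drawing, damaging zombies directly and flagging Head-bone hits as headshots with heavier damage.
; It builds the projectile's transform from the muzzle arrow toward the impact, but only after a successful zombie cast.
; A recoil timeline adds random yaw and pitch jitter.
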(event `FirePistol`
  (bind _playerreference (`self.PlayerReference`))
  (`SkeletalMeshComponent.PlayAnimation` (`self.InteractableSkeletalMesh`) "/Game/MilitaryWeapSilver/Weapons/Animations/Fire_Pistol_W.Fire_Pistol_W" false)
  (bind _spawntransfrom (`self.BulletTrace`))
  (`|SpawnActorFromClass` "/Game/Blueprints/Projectiles/BP_PistolProjectile.BP_PistolProjectile_C" _spawntransfrom "AlwaysSpawn" "OverrideRootScale" null null)
  (`Timeline|RecoilAnime` :!via `PlayFromStart`
    (:`Update`
      (`Pawn.AddControllerYawInput` _playerreference (`KismetMathLibrary.RandomFloatInRange` -0.15 0.15))
      (`Pawn.AddControllerPitchInput` _playerreference (`KismetMathLibrary.RandomFloatInRange` 0.15 -0.15)))))

(fn `BulletTrace`
  (returns (SpawnTransfrom :type "Transform Structure"))
  (bind _returnvalue (`SceneComponent.K2_GetComponentLocation` (`self.Arrow`)))
  (bind _followcamera (`/Game/Blueprints/Core/Player/BP_Player.FollowCamera` (`self.PlayerReference`)))
  (bind _returnvalue_2 (`SceneComponent.K2_GetComponentLocation` _followcamera))
  (bind (_outhit _returnvalue_3) (`KismetSystemLibrary.LineTraceSingle` :`Start` _returnvalue_2 :`End` (+ _returnvalue_2 (* (`SceneComponent.GetForwardVector` _followcamera) 15000.0)) :`TraceChannel` "TraceTypeQuery1" :`DrawDebugType` "ForDuration" :`DrawTime` 2.0))
  (bind (_bblockinghit _binitialoverlap _time _distance _location _impactpoint _normal _impactnormal _physmat _hitactor _hitcomponent _hitbonename) (`GameplayStatics.BreakHitResult` _outhit))
  (bind _asbp_master_zombie (cast `/Game/Blueprints/Core/Enemy/BP_MasterZombie` _hitactor))
  (if (== _hitbonename "Head")
    (set `/Game/Blueprints/Core/Enemy/BP_MasterZombie.isHeadshot?` true _asbp_master_zombie)
    (`/Game/Blueprints/Core/Enemy/BP_MasterZombie.AffectHealth` _asbp_master_zombie -100.0)
    (else
      (`/Game/Blueprints/Core/Enemy/BP_MasterZombie.AffectHealth` _asbp_master_zombie -25.0)))
  (`KismetSystemLibrary.PrintString` (`KismetStringLibrary.Conv_NameToString` _hitbonename))
  (return (`KismetMathLibrary.MakeTransform` _returnvalue (select `bool` _returnvalue_3 :`false` (`SceneComponent.K2_GetComponentRotation` _followcamera) :`true` (`KismetMathLibrary.FindLookAtRotation` _returnvalue _impactpoint)) (10.0 1.0 1.0))))

(fn `Interact`
  (params (PlayerReference :type "/Game/Blueprints/Core/Player/BP_Player Object Reference"))
  (`parent.Interact` PlayerReference)
  (`/Game/Blueprints/Core/Player/BP_Player.WeaponsPickup` PlayerReference))

(fn `UserConstructionScript`
  (`parent.UserConstructionScript`))