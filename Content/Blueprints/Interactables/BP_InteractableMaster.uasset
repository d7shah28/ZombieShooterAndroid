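; Base Blueprint for interactable objects that the player can highlight and interact with.
; A trigger adds or removes the object from BP_Player's interactions on overlap, and BeginPlay passes the description to its WBP_InteractionUi widget.
; ToggleHighlight switches custom depth on the skeletal and static meshes along with the widget's visibility.
; Interact stores the player reference and only prints a placeholder message.
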(event `self.ReceiveBeginPlay`
  (bind _aswbp_interaction_ui (cast `/Game/Blueprints/WidgetBlueprints/WBP_InteractionUi` (`WidgetComponent.GetUserWidgetObject` (`self.InteractableUi`))))
  (bind _output_get (set `self.InteractionUiReferecne` _aswbp_interaction_ui))
  (`/Game/Blueprints/WidgetBlueprints/WBP_InteractionUi.Set Description` _output_get (`self.Description`)))

(event `self.InteractableTrigger.OnComponentBeginOverlap`
  (params (OverlappedComponent :type "PrimitiveComponent Object Reference") (OtherActor :type "Actor Object Reference") (OtherComp :type "PrimitiveComponent Object Reference") (OtherBodyIndex :type Integer) (bFromSweep :type Boolean) (SweepResult :type "HitResult Structure (by ref)"))
  (bind _asbp_player (cast `/Game/Blueprints/Core/Player/BP_Player` OtherActor))
  (`/Game/Blueprints/Core/Player/BP_Player.AddInteraction` _asbp_player self))

(event `self.InteractableTrigger.OnComponentEndOverlap`
  (params (OverlappedComponent :type "PrimitiveComponent Object Reference") (OtherActor :type "Actor Object Reference") (OtherComp :type "PrimitiveComponent Object Reference") (OtherBodyIndex :type Integer))
  (bind _asbp_player (cast `/Game/Blueprints/Core/Player/BP_Player` OtherActor))
  (`/Game/Blueprints/Core/Player/BP_Player.RemoveInteraction` _asbp_player self))

(fn `Interact`
  (params (PlayerReference :type "/Game/Blueprints/Core/Player/BP_Player Object Reference"))
  (set `self.PlayerReference` PlayerReference)
  (`KismetSystemLibrary.PrintString` "Hello"))

(fn `ToggleHighlight`
  (params (`Highlight?` :type Boolean))
  (`PrimitiveComponent.SetRenderCustomDepth` (`self.InteractableSkeletalMesh`) `Highlight?`)
  (`PrimitiveComponent.SetRenderCustomDepth` (`self.InteractableMesh`) `Highlight?`)
  (`SceneComponent.SetVisibility` (`self.InteractableUi`) `Highlight?` false))

(fn `UserConstructionScript`)