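; BP_InteractableMaster_Child is an interactable that moves the player's camera to itself and back when used.
; Its Interact override calls the parent logic, then a FlipFlop alternates each use between blending player 0's view target to this actor and back to the BP_Player character.
; Both switches use a timed ease-in-out blend, while BeginPlay and the construction script add no logic of their own.
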(fn `Interact`
  (params (PlayerReference :type "/Game/Blueprints/Core/Player/BP_Player Object Reference"))
  (`parent.Interact` PlayerReference)
  (`/Engine/EditorBlueprintResources/StandardMacros.FlipFlop`
    (:`A`
      (`PlayerController.SetViewTargetWithBlend` (`GameplayStatics.GetPlayerController` 0) self 1.0 "VTBlend_EaseInOut" 1.0 false))
    (:`B`
      (`PlayerController.SetViewTargetWithBlend` (`GameplayStatics.GetPlayerController` 0) (cast `/Game/Blueprints/Core/Player/BP_Player` (`GameplayStatics.GetPlayerCharacter` 0) :!pure true) 1.0 "VTBlend_EaseInOut" 1.0 false))))

(fn `UserConstructionScript`
  (`parent.UserConstructionScript`))