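; BP_Item is a world pickup actor that places an item into the player's inventory.
; On BeginPlay it fills an unset ItemObject from GetDefaultItem, which returns nothing here and appears intended for child Blueprints to override.
; When BP_Player overlaps its Sphere, it passes ItemObject to the player's inventory component through TryAddItem and destroys itself only if the add succeeds.
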(event `self.ReceiveBeginPlay`
  (`/Engine/EditorBlueprintResources/StandardMacros.IsValid` (`self.ItemObject`)
    (:`Is Not Valid`
      (bind _itemobject (`self.GetDefaultItem`))
      (set `self.ItemObject` _itemobject))))

(event `self.Sphere.OnComponentBeginOverlap`
  (params (OverlappedComponent :type "PrimitiveComponent Object Reference") (OtherActor :type "Actor Object Reference") (OtherComp :type "PrimitiveComponent Object Reference") (OtherBodyIndex :type Integer) (bFromSweep :type Boolean) (SweepResult :type "HitResult Structure (by ref)"))
  (bind _asbp_player (cast `/Game/Blueprints/Core/Player/BP_Player` OtherActor))
  (bind _added (`/Game/Blueprints/Inventory/BP_InventoryComponent.TryAddItem` (`/Game/Blueprints/Core/Player/BP_Player.BP_InventoryComponent` _asbp_player) (`self.ItemObject`)))
  (if _added
    (`self.K2_DestroyActor`)))

(fn `GetDefaultItem`
  (returns (ItemObject :type "/Game/Blueprints/Inventory/BP_ItemObject Object Reference"))
  (return null))

(fn `UserConstructionScript`)