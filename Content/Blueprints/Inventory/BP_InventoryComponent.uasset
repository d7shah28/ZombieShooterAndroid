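; Grid inventory component that stores multi-tile items in a flat Items array sized Columns × Rows at BeginPlay.
; TryAddItem loops over slots, calling IsRoomAvailabe and AddItemAt, though as wired it does not branch on the room check.
; A ForEachIndex macro derives tiles from item dimensions and top-left index for both checking and writing, using tile/index conversion helpers.
; AddItemAt writes the item into each tile and sets IsDirty.
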(event `self.ReceiveBeginPlay`
  (`KismetArrayLibrary.Array_Resize` (`self.Items`) (* (`self.Columns`) (`self.Rows`))))

(fn `AddItemAt`
  (params (ItemObject :type "/Game/Blueprints/Inventory/BP_ItemObject Object Reference") (TopLeftIndex :type Integer))
  (bind _tile (`self.ForEachIndex` ItemObject TopLeftIndex)
    (:`LoopBody`
      (`KismetArrayLibrary.Array_Set` (`self.Items`) (`self.TileToIndex` _tile) (`local.ItemObject`)))
    (:`Completed`
      (set `self.isDirty` true))))

(fn `GetItemAtIndex`
  (params (Index :type Integer))
  (returns (Valid :type Boolean) (ItemObject :type "/Game/Blueprints/Inventory/BP_ItemObject Object Reference"))
  (bind _items (`self.Items`))
  (if (`KismetArrayLibrary.Array_IsValidIndex` _items Index)
    (return true (`|GetArrayItem` _items Index))
    (else
      (return false null))))

(fn `IndexToTile`
  (params (Index :type Integer))
  (returns (Tile :type "/Game/Blueprints/Inventory/S_Tile Structure"))
  (return (make `/Game/Blueprints/Inventory/S_Tile` (mod Index (`self.Columns`)) (/ Index (`self.Columns`)))))

(fn `isRoomAvailabe`
  (params (ItemObject :type "/Game/Blueprints/Inventory/BP_ItemObject Object Reference") (TopLeftIndex :type Integer))
  (returns (Result :type Boolean))
  (`|ExecutionSequence`
    (:`then_0`
      (bind _tile (`self.ForEachIndex` (`local.ItemObject`) (`local.TopLeftIndex`))
        (:`LoopBody`
          (`self.isTileValid` _tile
            (:`true`
              (bind (_valid _itemobject) (`self.GetItemAtIndex` (`self.TileToIndex` _tile)))
              (if _valid
                (if (`KismetSystemLibrary.IsValid` _itemobject)
                  (return false))
                (else
                  (return false))))
            (:`false`
              (return false))))))
    (:`then_1`
      (return true))))

(fn `TileToIndex`
  (params (Tile :type "/Game/Blueprints/Inventory/S_Tile Structure"))
  (returns (Index :type Integer))
  (bind (_x _y) (break `/Game/Blueprints/Inventory/S_Tile` Tile))
  (return (+ _x (* _y (`self.Columns`)))))

(fn `TryAddItem`
  (params (ItemObject :type "/Game/Blueprints/Inventory/BP_ItemObject Object Reference"))
  (returns (Added :type Boolean))
  (`/Engine/EditorBlueprintResources/StandardMacros.IsValid` ItemObject
    (:`Is Valid`
      (for (_ _array_index) (`self.Items`)
        (`self.isRoomAvailabe` (`local.ItemObject`) _array_index)
        (`self.AddItemAt` (`local.ItemObject`) _array_index)
        (return true))
      (return false))))