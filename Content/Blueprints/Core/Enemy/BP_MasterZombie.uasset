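; Base zombie enemy with modular limb meshes slaved to the main mesh, built for per-limb dismemberment.
; A sphere overlap toggles Attack, and right-hand overlaps call AffectHealth on the player.
; Limb functions map hit bones to meshes, track health and swap depleted limbs for launched physics actors.
; Point damage, limb-health setup and the death check are unwired, so dismemberment and the animated Death event are never triggered here.
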(event `self.ReceiveBeginPlay`)

(event `self.ReceivePointDamage`
  (params (Damage :type "Float (single-precision)") (DamageType :type "DamageType Object Reference") (HitLocation :type "Vector Structure") (HitNormal :type "Vector Structure") (HitComponent :type "PrimitiveComponent Object Reference") (BoneName :type Name) (ShotFromDirection :type "Vector Structure") (InstigatedBy :type "Controller Object Reference") (DamageCauser :type "Actor Object Reference") (HitInfo :type "HitResult Structure (by ref)")))

(event `Dismember`
  (params (DismemberPart :type "SkinnedMeshComponent Object Reference"))
  (`SkinnedMeshComponent.SetLeaderPoseComponent` DismemberPart null false)
  (`KismetSystemLibrary.Delay` 0.2)
  (`PrimitiveComponent.SetSimulatePhysics` DismemberPart true))

(event `DismemberLimb`
  (params (LimbToSpawn :type "SkeletalMesh Object Reference") (MeshToDestroy :type "SkeletalMeshComponent Object Reference"))
  (bind _returnvalue (`KismetMathLibrary.RandomFloatInRange` -250.0 250.0))
  (`ActorComponent.K2_DestroyComponent` MeshToDestroy)
  (bind _returnvalue_2 (`|SpawnActorFromClass` "/Game/Blueprints/Core/Enemy/BP_DismemberedLimb.BP_DismemberedLimb_C" (`SceneComponent.K2_GetComponentToWorld` (`self.Mesh`)) "AlwaysSpawn" "OverrideRootScale" null null))
  (bind _skeletalmesh (`/Game/Blueprints/Core/Enemy/BP_DismemberedLimb.SkeletalMesh` _returnvalue_2))
  (`SkinnedMeshComponent.SetSkinnedAssetAndUpdate` _skeletalmesh LimbToSpawn true)
  (`PrimitiveComponent.SetCollisionEnabled` _skeletalmesh "PhysicsOnly")
  (`PrimitiveComponent.SetSimulatePhysics` _skeletalmesh true)
  (`PrimitiveComponent.AddImpulse` _skeletalmesh (`KismetMathLibrary.MakeVector` _returnvalue _returnvalue (`KismetMathLibrary.RandomFloatInRange` 500.0 700.0)) "None" false))

(event `Death`
  (bind _mesh (`self.Mesh`))
  (if (`self.isDead?`)
    (`BrainComponent.StopLogic` (`AIController.BrainComponent` (`AIBlueprintHelperLibrary.GetAIController` self)) "Margaya")
    (if (`self.isHeadshot?`)
      (`SkeletalMeshComponent.PlayAnimation` _mesh "/Game/Characters/ZombieAnimations/Flying_Back_Death.Flying_Back_Death" false)
      (else
        (`SkeletalMeshComponent.PlayAnimation` _mesh "/Game/Characters/ZombieAnimations/Zombie_Death.Zombie_Death" false)))
    (`KismetSystemLibrary.Delay` 3.5)
    (`self.K2_DestroyActor`)))

(event `self.RightHandCollision.OnComponentBeginOverlap`
  (params (OverlappedComponent :type "PrimitiveComponent Object Reference") (OtherActor :type "Actor Object Reference") (OtherComp :type "PrimitiveComponent Object Reference") (OtherBodyIndex :type Integer) (bFromSweep :type Boolean) (SweepResult :type "HitResult Structure (by ref)"))
  (bind _asbp_player (cast `/Game/Blueprints/Core/Player/BP_Player` (`|GetArrayItem` (`self.GetOverlappingActors` OtherActor "/Game/Blueprints/Core/Player/BP_Player.BP_Player_C"))))
  (`/Game/Blueprints/Core/Player/BP_Player.AffectHealth` _asbp_player 25.0))

(event `self.Sphere.OnComponentBeginOverlap`
  (params (OverlappedComponent :type "PrimitiveComponent Object Reference") (OtherActor :type "Actor Object Reference") (OtherComp :type "PrimitiveComponent Object Reference") (OtherBodyIndex :type Integer) (bFromSweep :type Boolean) (SweepResult :type "HitResult Structure (by ref)"))
  (cast `/Game/Blueprints/Core/Player/BP_Player` OtherActor)
  (set `self.Attack?` true))

(event `self.Sphere.OnComponentEndOverlap`
  (params (OverlappedComponent :type "PrimitiveComponent Object Reference") (OtherActor :type "Actor Object Reference") (OtherComp :type "PrimitiveComponent Object Reference") (OtherBodyIndex :type Integer))
  (cast `/Game/Blueprints/Core/Player/BP_Player` OtherActor)
  (set `self.Attack?` false))

(fn `AffectHealth`
  (params (DeltaHealth :type "Float (double-precision)"))
  (bind _output_get (set `self.CurrentHealth` (+ DeltaHealth (`self.CurrentHealth`))))
  (`KismetSystemLibrary.PrintString` (`KismetStringLibrary.Conv_DoubleToString` _output_get)))

(fn `DamageLimb`
  (params (Limb :type "SkeletalMeshComponent Object Reference"))
  (returns (`LimbDestroyed?` :type Boolean))
  (bind _limb (`local.Limb`))
  (bind (_value _returnvalue) (`BlueprintMapLibrary.Map_Find` (`self.LimbHealth`) Limb))
  (bind _returnvalue_2 (- _value (`self.Damage`)))
  (if (and (> _value 0.0) _returnvalue)
    (`BlueprintMapLibrary.Map_Add` (`self.LimbHealth`) (`local.Limb`) (`KismetMathLibrary.SelectFloat` _returnvalue_2 0.0 (> _returnvalue_2 0.0)))
    (if (<= (`BlueprintMapLibrary.Map_Find` (`self.LimbHealth`) (`local.Limb`)) 0.0)
      (`self.DismemberLimb` (`SkinnedMeshComponent.SkeletalMesh` _limb) _limb)
      (return true)
      (else
        (return false)))))

(fn `GetDamagedLimb`
  (returns (LimbToDismember :type "SkeletalMeshComponent Object Reference") (`HitDismember?` :type Boolean))
  (bind _copzombieleftleg (`self.CopZombieLeftLeg`))
  (bind _bone_name (`self.Bone Name`))
  (bind _copzombierighthand (`self.CopZombieRightHand`))
  (bind _bone_name_2 (`self.Bone Name`))
  (bind _bone_name_3 (`self.Bone Name`))
  (bind _copzombielefthand (`self.CopZombieLeftHand`))
  (bind _copzombierightleg (`self.CopZombieRightLeg`))
  (bind _bone_name_4 (`self.Bone Name`))
  (`/Engine/EditorBlueprintResources/StandardMacros.IsValid` _copzombierightleg
    (:`Is Valid`
      (if (or (`SkinnedMeshComponent.BoneIsChildOf` _copzombierightleg _bone_name_4 "RightUpLeg") (== _bone_name_4 "RightUpLeg"))
        (`KismetSystemLibrary.PrintString` (`KismetStringLibrary.Conv_NameToString` _bone_name_4))
        (return (`self.CopZombieRightLeg`) true)
        (else
          _)))
    (:`Is Not Valid`
      _))
  (`/Engine/EditorBlueprintResources/StandardMacros.IsValid` _copzombieleftleg
    (:`Is Valid`
      (if (or (`SkinnedMeshComponent.BoneIsChildOf` _copzombieleftleg _bone_name "LeftUpLeg") (== _bone_name "LeftUpLeg"))
        (`KismetSystemLibrary.PrintString` (`KismetStringLibrary.Conv_NameToString` _bone_name))
        (return (`self.CopZombieLeftLeg`) true)
        (else
          _)))
    (:`Is Not Valid`
      _))
  (`/Engine/EditorBlueprintResources/StandardMacros.IsValid` _copzombierighthand
    (:`Is Valid`
      (if (or (`SkinnedMeshComponent.BoneIsChildOf` _copzombierighthand _bone_name_2 "RightArm") (== _bone_name_2 "RightArm"))
        (`KismetSystemLibrary.PrintString` (`KismetStringLibrary.Conv_NameToString` _bone_name_2))
        (return (`self.CopZombieRightHand`) true)
        (else
          _)))
    (:`Is Not Valid`
      _))
  (`/Engine/EditorBlueprintResources/StandardMacros.IsValid` _copzombielefthand
    (:`Is Valid`
      (if (or (`SkinnedMeshComponent.BoneIsChildOf` _copzombielefthand _bone_name_3 "LefttArm") (== _bone_name_3 "LefttArm"))
        (`KismetSystemLibrary.PrintString` (`KismetStringLibrary.Conv_NameToString` _bone_name_3))
        (return (`self.CopZombieLeftHand`) true)))))

(fn `UserConstructionScript`
  (`SkinnedMeshComponent.SetLeaderPoseComponent` (`self.CopZombieRightLeg`) (`self.Mesh`) false)
  (`SkinnedMeshComponent.SetLeaderPoseComponent` (`self.CopZombieRightHand`) (`self.Mesh`) false)
  (`SkinnedMeshComponent.SetLeaderPoseComponent` (`self.CopZombieLeftHand`) (`self.Mesh`) false)
  (`SkinnedMeshComponent.SetLeaderPoseComponent` (`self.CopZombieTorso`) (`self.Mesh`) false)
  (`SkinnedMeshComponent.SetLeaderPoseComponent` (`self.CopZombieLeftLeg`) (`self.Mesh`) false))